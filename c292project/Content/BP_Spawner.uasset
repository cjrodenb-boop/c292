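; Spawner actor that creates BP_Cube actors at tagged target points in the level.
; On BeginPlay it finds every TargetPoint tagged "SpawnPoint" and spawns a cube at each one's transform.
; A SpawnThing event spawns a single cube at the spawner's own root location.
; Unconnected leftover logic would spawn cubes at all or a random entry of a SpawnPosition array.
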(event `self.ReceiveBeginPlay`
  (bind _outactors (`GameplayStatics.GetAllActorsOfClassWithTag` "/Script/Engine.TargetPoint" "SpawnPoint"))
  (for _array_element _outactors
    (`|SpawnActorFromClass` "/Game/BP_Cube.BP_Cube_C" (`self.GetTransform` _array_element) "Undefined" "MultiplyWithRoot" null null)))

(event `Spawn Thing`
  ;[1 1 1] spawner
  (`|SpawnActorFromClass` "/Game/BP_Cube.BP_Cube_C" (`KismetMathLibrary.Conv_VectorToTransform` (`SceneComponent.K2_GetComponentLocation` (`self.DefaultSceneRoot`))) "Undefined" "MultiplyWithRoot" null null))

(fn `UserConstructionScript`)