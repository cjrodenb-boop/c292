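; BP_Trigger is an overlap trigger that lets the player toggle a Lightbulb actor's visibility with F.
; When BP_FirstPersonCharacter enters, it hides the bulb, sets the character's LightOn to true and enables player 0 input; exit disables input.
; A FlipFlop on F alternately shows and hides the bulb, setting LightOn to true on both branches, so this Blueprint never clears that flag.
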(event `self.ReceiveActorBeginOverlap`
  (params (OtherActor :type "Actor Object Reference"))
  (bind _asbp_first_person_character (cast `/Game/FirstPerson/Blueprints/BP_FirstPersonCharacter` OtherActor))
  (set `/Game/FirstPerson/Blueprints/BP_FirstPersonCharacter.Light On?` true _asbp_first_person_character)
  (`self.SetActorHiddenInGame` (`self.Lightbulb`) true)
  (`self.EnableInput` (`GameplayStatics.GetPlayerController` 0)))

(event `Key|F`
  (params (Key :type "Key Structure"))
  (:`Pressed`
    (`/Engine/EditorBlueprintResources/StandardMacros.FlipFlop`
      (:`A`
        (`self.SetActorHiddenInGame` (`self.Lightbulb`) false)
        (set `/Game/FirstPerson/Blueprints/BP_FirstPersonCharacter.Light On?` true (stale `self.ReceiveActorBeginOverlap` _asbp_first_person_character)))
      (:`B`
        (`self.SetActorHiddenInGame` (`self.Lightbulb`) true)
        (set `/Game/FirstPerson/Blueprints/BP_FirstPersonCharacter.Light On?` true (stale `self.ReceiveActorBeginOverlap` _asbp_first_person_character))))))

(event `self.ReceiveActorEndOverlap`
  (params (OtherActor :type "Actor Object Reference"))
  (cast `/Game/FirstPerson/Blueprints/BP_FirstPersonCharacter` OtherActor)
  (`self.DisableInput` (`GameplayStatics.GetPlayerController` 0)))

(fn `UserConstructionScript`)